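; Bunny actor that wanders in timeline-driven moves along random horizontal directions, starting on BeginPlay.
; Each direction gets three moves separated by short delays, lerping position at its starting height while blending yaw, before a new direction is picked.
; Targets are the direction scaled by move count, measured from world origin rather than the bunny.
; StopMoving halts the timeline; the cached MouseGrabPawn is unused here.
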(event Custom|ContinueMoving
  (bind _returnvalue (Math|Random|RandomUnitVector))
  (bind _returnvalue_2 (Transformation|GetActorRotation))
  (bind _returnvalue_3 (Transformation|GetActorRotation))
  (Variables|Default|SetNumberOfLoop 0 :!label _label)
  (Variables|Default|SetRandomVector (Math|Vector|Normalize (Math|Vector|MakeVector (.x _returnvalue) (.y _returnvalue) 0.0) 1e-05))
  (if (> (Variables|Default|GetNumberOfLoop) 2) :!label _label_2
    (goto _label)
    (else
      (Variables|Default|SetNumberOfLoop (+ (Variables|Default|GetNumberOfLoop) 1))
      (Variables|Default|SetRndomRotation (Math|Rotator|MakeRotator (.roll _returnvalue_3) (.pitch _returnvalue_3) 0.0))
      (bind _alpha (Timeline|Timeline_0 PlayFromStart)
        (:Update
          (Transformation|SetActorLocation (Math|Vector|Lerp(Vector) (Variables|Default|GetJumpedLocation) (Math|Vector|MakeVector (.x (* (* (Variables|Default|GetRandomVector) (Variables|Default|GetNumberOfLoop)) 4e+02)) (.y (* (* (Variables|Default|GetRandomVector) (Variables|Default|GetNumberOfLoop)) 4e+02)) (Variables|Default|GetZLocation)) _alpha) false false)
          (Variables|Default|SetNewLocation (Math|Vector|Lerp(Vector) (Variables|Default|GetJumpedLocation) (Math|Vector|MakeVector (.x (* (* (Variables|Default|GetRandomVector) (Variables|Default|GetNumberOfLoop)) 4e+02)) (.y (* (* (Variables|Default|GetRandomVector) (Variables|Default|GetNumberOfLoop)) 4e+02)) (Variables|Default|GetZLocation)) _alpha))
          (Transformation|SetActorRotation (Math|Rotator|Lerp(Rotator) (Transformation|GetActorRotation) (Math|Rotator|MakeRotator (.roll _returnvalue_2) (.pitch _returnvalue_2) (.yaw (Math|Rotator|MakeRotfromZ (Variables|Default|GetRandomVector)))) _alpha)))
        (:Finished
          (Variables|Default|SetJumpedLocation (Transformation|GetActorLocation))
          (Utilities|FlowControl|Delay 0.2)
          (goto _label_2))))))

(event Custom|StartMoving
  (bind _returnvalue (Math|Random|RandomUnitVector))
  (bind _returnvalue_2 (Transformation|GetActorRotation))
  (bind _returnvalue_3 (Transformation|GetActorRotation))
  (Variables|Default|SetRandomVector (Math|Vector|Normalize (Math|Vector|MakeVector (.x _returnvalue) (.y _returnvalue) 0.0) 1e-05) :!label _label)
  (if (> (Variables|Default|GetNumberOfLoop) 2) :!label _label_2
    (Variables|Default|SetNumberOfLoop 0)
    (goto _label)
    (else
      (Variables|Default|SetNumberOfLoop (+ (Variables|Default|GetNumberOfLoop) 1))
      (Variables|Default|SetRndomRotation (Math|Rotator|MakeRotator (.roll _returnvalue_3) (.pitch _returnvalue_3) 0.0))
      (bind _alpha (Timeline|Timeline_0 PlayFromStart)
        (:Update
          (Transformation|SetActorLocation (Math|Vector|Lerp(Vector) (Variables|Default|GetJumpedLocation) (Math|Vector|MakeVector (.x (* (* (Variables|Default|GetRandomVector) (Variables|Default|GetNumberOfLoop)) 4e+02)) (.y (* (* (Variables|Default|GetRandomVector) (Variables|Default|GetNumberOfLoop)) 4e+02)) (Variables|Default|GetZLocation)) _alpha) false false)
          (Variables|Default|SetNewLocation (Math|Vector|Lerp(Vector) (Variables|Default|GetJumpedLocation) (Math|Vector|MakeVector (.x (* (* (Variables|Default|GetRandomVector) (Variables|Default|GetNumberOfLoop)) 4e+02)) (.y (* (* (Variables|Default|GetRandomVector) (Variables|Default|GetNumberOfLoop)) 4e+02)) (Variables|Default|GetZLocation)) _alpha))
          (Transformation|SetActorRotation (Math|Rotator|Lerp(Rotator) (Transformation|GetActorRotation) (Math|Rotator|MakeRotator (.roll _returnvalue_2) (.pitch _returnvalue_2) (.yaw (Math|Rotator|MakeRotfromZ (Variables|Default|GetRandomVector)))) _alpha)))
        (:Finished
          (Variables|Default|SetJumpedLocation (Transformation|GetActorLocation))
          (Utilities|FlowControl|Delay 0.2)
          (goto _label_2))))))

(event Custom|StopMoving
  (bind _returnvalue (Math|Random|RandomUnitVector))
  (bind _returnvalue_2 (Transformation|GetActorRotation))
  (bind _returnvalue_3 (Transformation|GetActorRotation))
  (bind _alpha (Timeline|Timeline_0 Stop)
    (:Update
      (Transformation|SetActorLocation (Math|Vector|Lerp(Vector) (Variables|Default|GetJumpedLocation) (Math|Vector|MakeVector (.x (* (* (Variables|Default|GetRandomVector) (Variables|Default|GetNumberOfLoop)) 4e+02)) (.y (* (* (Variables|Default|GetRandomVector) (Variables|Default|GetNumberOfLoop)) 4e+02)) (Variables|Default|GetZLocation)) _alpha) false false)
      (Variables|Default|SetNewLocation (Math|Vector|Lerp(Vector) (Variables|Default|GetJumpedLocation) (Math|Vector|MakeVector (.x (* (* (Variables|Default|GetRandomVector) (Variables|Default|GetNumberOfLoop)) 4e+02)) (.y (* (* (Variables|Default|GetRandomVector) (Variables|Default|GetNumberOfLoop)) 4e+02)) (Variables|Default|GetZLocation)) _alpha))
      (Transformation|SetActorRotation (Math|Rotator|Lerp(Rotator) (Transformation|GetActorRotation) (Math|Rotator|MakeRotator (.roll _returnvalue_2) (.pitch _returnvalue_2) (.yaw (Math|Rotator|MakeRotfromZ (Variables|Default|GetRandomVector)))) _alpha)))
    (:Finished
      (Variables|Default|SetJumpedLocation (Transformation|GetActorLocation))
      (Utilities|FlowControl|Delay 0.2)
      (if (> (Variables|Default|GetNumberOfLoop) 2) :!label _label
        (Variables|Default|SetNumberOfLoop 0)
        (Variables|Default|SetRandomVector (Math|Vector|Normalize (Math|Vector|MakeVector (.x _returnvalue) (.y _returnvalue) 0.0) 1e-05))
        (goto _label)
        (else
          (Variables|Default|SetNumberOfLoop (+ (Variables|Default|GetNumberOfLoop) 1))
          (Variables|Default|SetRndomRotation (Math|Rotator|MakeRotator (.roll _returnvalue_3) (.pitch _returnvalue_3) 0.0))
          (Timeline|Timeline_0 PlayFromStart))))))

(event EventBeginPlay
  (bind _outactors (Actor|GetAllActorsOfClass "/Game/BP/MouseGrabPawn.MouseGrabPawn_C"))
  (Variables|Default|SetMouseGrabPawn (Utilities|Array|Get(acopy) _outactors))
  (Variables|Default|SetZLocation (.z (Transformation|GetActorLocation)))
  (Variables|Default|SetJumpedLocation (Transformation|GetActorLocation))
  (CallFunction|StartMoving))

(fn ConstructionScript)